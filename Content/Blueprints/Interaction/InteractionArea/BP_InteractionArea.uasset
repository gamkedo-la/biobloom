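; BP_InteractionArea is an interaction area actor that relays focus changes to the parent actor it is attached to as a child actor.
; ToggleFocus stores the Focused state and forwards it to the parent through a ToggleFocusMessage call.
; It then requests the parent's interaction widget reference and, if valid, shows that widget while focused and hides it otherwise.
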(event `ToggleFocus`
  (params (Focused :type Boolean))
  (set `self.Focused` Focused)
  (message `/Game/Blueprints/Interaction/InteractionArea/BI_Interaction.ToggleFocus` (`self.GetParentActor`) (`self.Focused`))
  (bind _ref (message `/Game/Blueprints/Interaction/InteractionArea/BI_Interaction.GetInteractionWidgetRef` (`self.GetParentActor`)))
  (if (`KismetSystemLibrary.IsValid` _ref)
    (`SceneComponent.SetHiddenInGame` _ref (not (`self.Focused`)) false)))

(fn `UserConstructionScript`)