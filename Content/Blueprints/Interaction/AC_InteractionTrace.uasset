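; Interaction component that traces from the player camera each tick to find and focus BP_InteractionArea actors.
; LineTrace acts only when the hit actor changes or the trace misses, and TraceInteractionarea toggles focus on the old and new areas.
; TryToInteract sends zero-duration interactions through InteractOnServer to InteractWithMessage on the area's parent actor.
; For longer interactions it only stores InteractDuration, with no hold logic here.
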(event `self.ReceiveTick`
  (params (DeltaSeconds :type "Float (single-precision)"))
  (`self.LineTrace`))

(event `TryToInteract`
  (params (In :type Boolean))
  (if In
    ;[1 1 1] Player is looking at interaction area
    (if (`self.IsTracingInteractionArea`)
      ;[1 1 1] Store the interact duration of that object for later
      (bind _output_get (set `self.Interact Duration` (`/Game/Blueprints/Interaction/InteractionArea/BP_InteractionArea.InteractDuration` (`self.FocusedInteractionArea`))))
      ;[1 1 1] Interaction of length 0 is instant, otherwise it requires a held key press
      (if (not (> _output_get 0.0))
        (`self.InteractOnServer` (`self.FocusedInteractionArea`))))))

(event `InteractOnServer`
  (params (InteractionArea :type "/Game/Blueprints/Interaction/InteractionArea/BP_InteractionArea Object Reference"))
  (message `/Game/Blueprints/Interaction/InteractionArea/BI_Interaction.InteractWith` (`Actor.GetParentActor` InteractionArea)))

(fn `LineTrace`
  (bind _returnvalue (`GameplayStatics.GetPlayerCameraManager` 0))
  (bind _returnvalue_2 (`PlayerCameraManager.GetCameraLocation` _returnvalue))
  ;[1 1 1] Trace from the player camera forward trace length amount, and line trace to see what we hit
  ;;[1 1 1] Perform Line Trace
  (bind (_outhit _returnvalue_3) (`KismetSystemLibrary.LineTraceSingle` _returnvalue_2 (+ _returnvalue_2 (* (`KismetMathLibrary.GetForwardVector` (`Actor.K2_GetActorRotation` _returnvalue)) (`self.Length`))) "TraceTypeQuery1"))
  (if _returnvalue_3
    (bind (_bblockinghit _binitialoverlap _time _distance _location _impactpoint _normal _impactnormal _physmat _hitactor) (`GameplayStatics.BreakHitResult` _outhit))
    ;;[1 1 1] Set focusedactor only once per unique.
    ;; Only continue when we receive a new focused actor, not the same one
    (if (!= (`self.FocusedActor`) _hitactor)
      (set `self.FocusedActor` _hitactor)
      ;;[1 1 1] Check traced actor has interactionarea
      (`self.TraceInteractionarea` (== (`GameplayStatics.GetObjectClass` _hitactor) "/Game/Blueprints/Interaction/InteractionArea/BP_InteractionArea.BP_InteractionArea_C")))
    (else
      (`self.TraceInteractionarea` false))))

(fn `TraceInteractionarea`
  (params (Trace :type Boolean))
  (bind _focusedinteractionarea (`self.FocusedInteractionArea`))
  (if Trace
    ;[1 1 1] We received a successful trace from LineTrace. This is also guarenteed to have BP_InteractionArea through linetrace
    (if (`self.IsTracingInteractionArea`)
      ;;[1 1 1] If we are switching off of a focused object to another focusable object, reset the one we are leaving
      (`/Game/Blueprints/Interaction/InteractionArea/BP_InteractionArea.ToggleFocus` (`self.FocusedInteractionArea`) false))
    (bind _asbp_interaction_area (cast `/Game/Blueprints/Interaction/InteractionArea/BP_InteractionArea` (`self.FocusedActor`)))
    (bind _output_get (set `self.FocusedInteractionArea` _asbp_interaction_area))
    (`/Game/Blueprints/Interaction/InteractionArea/BP_InteractionArea.ToggleFocus` _output_get true)
    (set `self.IsTracingInteractionArea` true)
    (else
      ;[1 1 1] Linetrace by channel failed, clear all focused
      (if (`self.IsTracingInteractionArea`)
        (set `self.IsTracingInteractionArea` false)
        (if (`KismetSystemLibrary.IsValid` _focusedinteractionarea)
          (`/Game/Blueprints/Interaction/InteractionArea/BP_InteractionArea.ToggleFocus` _focusedinteractionarea false)
          (set `self.FocusedInteractionArea` null)
          (set `self.FocusedActor` null))))))