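; Actor component that gives the first-person character a build mode for previewing and placing buildables loaded from a data table.
; While active, BuildCycle re-runs on a short delay, line tracing from the camera to position a collision-free ghost mesh.
; The ghost turns green on a trace hit and red otherwise, setting CanBuild.
; SpawnBuild spends the character's BuildMaterials to spawn the selected actor, without checking CanBuild itself.
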(event `self.ReceiveBeginPlay`
  (bind _asbp_first_person_character (cast `/Game/FirstPerson/Blueprints/BP_FirstPersonCharacter` (`self.GetOwner`)))
  (set `self.PlayerReference` _asbp_first_person_character)
  (set `self.Camera` null)
  (bind _outrownames (`DataTableFunctionLibrary.GetDataTableRowNames` "/Game/Blueprints/Gameplay/BaseBuilding/BuildablesDB.BuildablesDB"))
  (for _array_element _outrownames
    (bind _returnvalue (`|GetDataTableRow` "/Game/Blueprints/Gameplay/BaseBuilding/BuildablesDB.BuildablesDB" _array_element)
      (:`then`
        (`KismetArrayLibrary.Array_Add` (`self.Buildables`) _returnvalue)))))

(event `BuildDelay`
  (bind _buildghost (`self.BuildGhost`))
  (if (`self.BuildModeEnabled`)
    (`KismetSystemLibrary.Delay` 0.01)
    (`self.BuildCycle`)
    (else
      (set `self.BuildModeEnabled` false :!label _label)
      (set `self.CanBuild` false)
      (`/Engine/EditorBlueprintResources/StandardMacros.IsValid` _buildghost
        (:`Is Valid`
          (`/Game/FirstPerson/Blueprints/BP_FirstPersonCharacter.FP_Char_DestroyPassComponent` (`self.PlayerReference`) _buildghost))))))

(event `StopBuildMode`
  (goto _label))

(event `LaunchBuildMode`
  (if (`self.BuildModeEnabled`)
    (`self.StopBuildMode`)
    (else
      (set `self.BuildModeEnabled` true)
      (`self.BuildCycle`))))

(fn `BuildCycle`
  (bind (_buildtransform_location _buildtransform_rotation _buildtransform_scale) (`KismetMathLibrary.BreakTransform` (`self.BuildTransform`)))
  (bind _first_person_camera (`self.First Person Camera`))
  (bind _buildghost (`self.BuildGhost`))
  (bind _returnvalue (`SceneComponent.K2_GetComponentLocation` _first_person_camera))
  (bind (_output_mesh _output_tracechannel) (break `/Game/Blueprints/Gameplay/BaseBuilding/S_Buildables` (`|GetArrayItem` (`self.Buildables`) (`self.BuildID`))))
  (bind _returnvalue_2 (`KismetMathLibrary.GetForwardVector` (`SceneComponent.K2_GetComponentRotation` _first_person_camera)))
  (bind _asbp_first_person_character (cast `/Game/FirstPerson/Blueprints/BP_FirstPersonCharacter` (`GameplayStatics.GetPlayerCharacter` 0)))
  (set `self.First Person Camera` (`/Game/FirstPerson/Blueprints/BP_FirstPersonCharacter.FirstPersonCamera` _asbp_first_person_character))
  (bind (_outhit _returnvalue_3) (`KismetSystemLibrary.LineTraceSingle` (+ _returnvalue (* _returnvalue_2 (`self.BuildStart`))) (+ _returnvalue (* (`self.BuildEnd`) _returnvalue_2)) _output_tracechannel))
  (if _returnvalue_3
    (bind (_bblockinghit _binitialoverlap _time _distance _location _impactpoint _normal _impactnormal _physmat _hitactor _hitcomponent _hitbonename _bonename _hititem _elementindex _faceindex _tracestart _traceend) (`GameplayStatics.BreakHitResult` _outhit))
    (set `self.BuildTransform` (`KismetMathLibrary.MakeTransform` _impactpoint _buildtransform_rotation _buildtransform_scale))
    (`/Engine/EditorBlueprintResources/StandardMacros.IsValid` _buildghost
      (:`Is Valid`
        (`self.GiveBuildColor` true))
      (:`Is Not Valid`
        (`self.SpawnBuildGhost` :!label _label)))
    (else
      (set `self.BuildTransform` (`KismetMathLibrary.MakeTransform` _traceend _buildtransform_rotation _buildtransform_scale))
      (`/Engine/EditorBlueprintResources/StandardMacros.IsValid` _buildghost
        (:`Is Valid`
          (`self.GiveBuildColor` false))
        (:`Is Not Valid`
          (goto _label)))))
  (`self.BuildDelay`))

(fn `ChangeMesh`
  (bind _buildghost (`self.BuildGhost`))
  (bind _output_mesh (break `/Game/Blueprints/Gameplay/BaseBuilding/S_Buildables` (`|GetArrayItem` (`self.Buildables`) (`self.BuildID`))))
  (`/Engine/EditorBlueprintResources/StandardMacros.IsValid` _buildghost
    (:`Is Valid`
      (`StaticMeshComponent.SetStaticMesh` _buildghost _output_mesh))))

(fn `GiveBuildColor`
  (params (IsGreen :type Boolean))
  (set `self.CanBuild` IsGreen)
  (for _index (range (+ (`PrimitiveComponent.GetNumMaterials` (`self.BuildGhost`)) 1))
    (if IsGreen
      (`PrimitiveComponent.SetMaterial` (`self.BuildGhost`) _index "/Game/Art/Materials/Building/M_GreenColor.M_GreenColor")
      (else
        (`PrimitiveComponent.SetMaterial` (`self.BuildGhost`) _index "/Game/Art/Materials/Building/M_RedColor.M_RedColor"))))
  (`SceneComponent.K2_SetWorldTransform` (`self.BuildGhost`) (`self.BuildTransform`) false false))

(fn `SpawnBuild`
  (bind _playerreference (`self.PlayerReference`))
  (bind (_output_mesh _output_tracechannel _output_actor) (break `/Game/Blueprints/Gameplay/BaseBuilding/S_Buildables` (`|GetArrayItem` (`self.Buildables`) (`self.BuildID`))))
  (if (> (`|GetArrayItem` (`/Game/FirstPerson/Blueprints/BP_FirstPersonCharacter.BuildMaterials` _playerreference) (`self.BuildID`)) 0)
    (`/Engine/EditorBlueprintResources/StandardMacros.DecrementInt` (`|GetArrayItem` (`/Game/FirstPerson/Blueprints/BP_FirstPersonCharacter.BuildMaterials` _playerreference) (`self.BuildID`))
      (:`  `
        (`|SpawnActorFromClass` _output_actor (`self.BuildTransform`) "Undefined" "OverrideRootScale" null null)))))

(fn `SpawnBuildGhost`
  (bind _output_mesh (break `/Game/Blueprints/Gameplay/BaseBuilding/S_Buildables` (`|GetArrayItem` (`self.Buildables`) (`self.BuildID`))))
  (bind _returnvalue (`|AddComponentByClass` (`self.PlayerReference`) "/Script/Engine.StaticMeshComponent" false (`self.BuildTransform`)))
  (bind _output_get (set `self.BuildGhost` _returnvalue))
  (`StaticMeshComponent.SetStaticMesh` _output_get _output_mesh)
  (`PrimitiveComponent.SetCollisionEnabled` (`self.BuildGhost`) "NoCollision"))