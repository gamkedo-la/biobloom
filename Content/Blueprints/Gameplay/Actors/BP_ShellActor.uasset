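; BP_ShellActor builds a shell-texturing effect from stacked instances of a single Instanced Static Mesh.
; The construction script pushes shell count, base color and shape parameters such as density, length, curvature and noise range to the mesh materials.
; It then adds identity-transform instances in a ShellCount-driven loop, storing each loop index as per-instance custom data so the material can distinguish the layers.
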(event `self.ReceiveBeginPlay`)

(fn `CreateShells`
  (bind _instancedstaticmesh (`self.InstancedStaticMesh`))
  (for _index (range (+ (`self.ShellCount`) 1))
    (bind _returnvalue (`InstancedStaticMeshComponent.AddInstance` _instancedstaticmesh (`KismetMathLibrary.MakeTransform` (0.0 0.0 0.0)) false))
    (`InstancedStaticMeshComponent.SetCustomDataValue` (`self.InstancedStaticMesh`) _returnvalue 0 (`KismetMathLibrary.Conv_IntToDouble` _index) false))
  (message `AudioParameterControllerInterface.SetFloatParameter` (`PrimitiveComponent.GetMaterial` _instancedstaticmesh 0) "ShellCount" (`KismetMathLibrary.Conv_IntToDouble` (`self.ShellCount`))))

(fn `SetMaterialParameters`
  (bind _instancedstaticmesh (`self.InstancedStaticMesh`))
  (`MeshComponent.SetScalarParameterValueOnMaterials` _instancedstaticmesh "ShellCount" (`KismetMathLibrary.Conv_IntToDouble` (`self.ShellCount`)))
  (`MeshComponent.SetVectorParameterValueOnMaterials` _instancedstaticmesh "BaseColor" (`KismetMathLibrary.Conv_LinearColorToVector` (`self.BaseColor`)))
  (`MeshComponent.SetScalarParameterValueOnMaterials` _instancedstaticmesh "Density" (`self.Density`))
  (`MeshComponent.SetScalarParameterValueOnMaterials` _instancedstaticmesh "ShellLength" (`self.ShellLength`))
  (`MeshComponent.SetScalarParameterValueOnMaterials` _instancedstaticmesh "Thickness" (`self.Thickness`))
  (`MeshComponent.SetScalarParameterValueOnMaterials` _instancedstaticmesh "Curvature" (`self.Curvature`))
  (`MeshComponent.SetScalarParameterValueOnMaterials` _instancedstaticmesh "DisplacementStrength" (`self.DisplacementStrength`))
  (`MeshComponent.SetScalarParameterValueOnMaterials` _instancedstaticmesh "NoiseMin" (`self.NoiseMin`))
  (`MeshComponent.SetScalarParameterValueOnMaterials` _instancedstaticmesh "NoiseMax" (`self.NoiseMax`))
  (return))

(fn `UserConstructionScript`
  (`self.SetMaterialParameters`)
  (`self.CreateShells`))