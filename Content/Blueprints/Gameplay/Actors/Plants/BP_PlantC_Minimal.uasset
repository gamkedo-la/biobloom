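; Growable plant actor that ages on a looping timer and, once mature, can be harvested for a random count of ExoticSeedC seeds.
; Text renders show description, genus and age, colored by maturity and revealed on focus alongside a custom-depth highlight.
; Interaction flips InteractToggle through InteractOnServer, using its OnRep to harvest.
; Harvest gives seeds to player character 0 and resets the plant's age and maturity.
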(event `self.ReceiveBeginPlay`
  (set `self.SeedCount` (`KismetMathLibrary.FTrunc` (`KismetMathLibrary.RandomFloatInRange` 1.0 4.0)))
  (`KismetSystemLibrary.K2_SetTimerDelegate` (delegate `AgeIncrease`) 1.0 true)
  (`self.UpdateAgeDisplay`)
  (`TextRenderComponent.K2_SetText` (`self.Description Render`) (`KismetTextLibrary.Conv_StringToText` (`self.Description`)))
  (`TextRenderComponent.K2_SetText` (`self.Genus Render`) (`KismetTextLibrary.Conv_StringToText` (`self.Genus`))))

(event `AgeIncrease`
  (`self.IncreaseAge`)
  (`self.AgeIncreased`))

(event `/Game/Blueprints/Interaction/InteractionArea/BI_Interaction.ToggleFocus`
  (params (Focus :type Boolean))
  (`PrimitiveComponent.SetRenderCustomDepth` (`self.Plant`) Focus)
  (`WidgetComponent.SetDrawSize` (`self.Widget`) (200.0 50.0))
  (`SceneComponent.SetVisibility` (`self.Description Render`) Focus true)
  (`SceneComponent.SetVisibility` (`self.Genus Render`) Focus true)
  (`SceneComponent.SetVisibility` (`self.Age Render`) Focus true))

(event `/Game/Blueprints/Interaction/InteractionArea/BI_Interaction.InteractWith`
  (`self.InteractOnServer`))

(event `InteractOnServer`
  ;[1 1 1] Always set value to the opposite of what it currently is (a toggle)
  (set `self.InteractToggle` (not (`self.InteractToggle`))))

(event `SeedPickedUp`)

(fn `GetInteractionWidgetRef`
  (returns (Ref :type "WidgetComponent Object Reference"))
  (return (`self.Widget`)))

(fn `HandlePlantMaturity`
  (params (Age :type Integer))
  ;[1 1 1] Set Maturity Bool when reached
  (if (and (>= Age (`self.MatureAge`)) (not (`self.Mature`)))
    (set `self.Mature` true)
    (`TextRenderComponent.SetTextMaterial` (`self.Age Render`) "/Game/Art/Materials/TextBillboard_Green.TextBillboard_Green")))

(fn `HarvestPlant`
  (params (InputPin :type "/Game/FirstPerson/Blueprints/BP_FirstPersonCharacter Object Reference"))
  (if (`self.Mature`)
    (`/Game/FirstPerson/Blueprints/BP_FirstPersonCharacter.AddSeeds` InputPin (`self.SeedCount`) "ExoticSeedC")
    (set `self.Mature` false)
    (set `self.Age` 0)
    (`TextRenderComponent.SetTextMaterial` (`self.Age Render`) "/Game/Art/Materials/TextBillboard_Red.TextBillboard_Red")))

(fn `IncreaseAge`
  ;[1 1 1] Increment Age
  (bind _output_get (set `self.Age` (`KismetMathLibrary.Min` (+ (`self.Age`) 1) (`self.MaxAge`))))
  (`|ExecutionSequence`
    (:`then_0`
      (`self.HandlePlantMaturity` _output_get))
    (:`then_1`
      (`self.UpdateAgeDisplay`))))

(fn `OnRep_InteractToggle`
  (bind _asbp_first_person_character (cast `/Game/FirstPerson/Blueprints/BP_FirstPersonCharacter` (`GameplayStatics.GetPlayerCharacter` 0)))
  (`self.HarvestPlant` _asbp_first_person_character))

(fn `UpdateAgeDisplay`
  ;[1 1 1] UpdateAge
  (`TextRenderComponent.K2_SetText` (`self.Age Render`) (`|FormatText` "{age} / {maxAge}" (`KismetTextLibrary.Conv_IntToText` (`self.Age`)) (`KismetTextLibrary.Conv_IntToText` (`self.MaxAge`)))))

(fn `UserConstructionScript`)