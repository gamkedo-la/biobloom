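; Interactable request computer actor that highlights via custom depth when focused and opens a request-panel HUD widget on interaction.
; Interact calls InteractOnServer, which flips InteractToggle purely as a replication trigger.
; Its OnRep, ignoring the value, shows the panel on player character 0's HUD and stores the widget reference, so display is not limited to the interacting player.
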(event `/Game/Blueprints/Interaction/InteractionArea/BI_Interaction.ToggleFocus`
  (params (Focus :type Boolean))
  (`PrimitiveComponent.SetRenderCustomDepth` (`self.request_computer`) Focus))

(event `/Game/Blueprints/Interaction/InteractionArea/BI_Interaction.InteractWith`
  (`self.InteractOnServer`))

(event `InteractOnServer`
  ;[1 1 1] Always set value to the opposite of what it currently is (a toggle)
  (set `self.InteractToggle` (not (`self.InteractToggle`))))

(fn `GetInteractionWidgetRef`
  (returns (Ref :type "WidgetComponent Object Reference"))
  (return (`self.Widget`)))

(fn `OnRep_InteractToggle`
  (bind _asbp_first_person_character (cast `/Game/FirstPerson/Blueprints/BP_FirstPersonCharacter` (`GameplayStatics.GetPlayerCharacter` 0)))
  (`/Game/FirstPerson/Blueprints/BP_FirstPersonCharacter.ShowHudElement` _asbp_first_person_character "/Game/Blueprints/Interaction/WB_Minimal_InteractionPanelPanel_RequestComputer.WB_Minimal_InteractionPanelPanel_RequestComputer_C")
  (set `self.Request_Panel` (`/Game/FirstPerson/Blueprints/BP_FirstPersonCharacter.UserWidgetCurrentHudWidget` _asbp_first_person_character)))

(fn `UserConstructionScript`)